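; Weapon_Base is a weapon Blueprint whose FireBullet event fires a shot along the player's ThirdPersonCharacter camera aim.
; It spawns a Bullet_Base at the mesh's Muzzle socket and sets its velocity along FollowCamera's forward vector.
; A separate camera line trace on Visibility, drawn with persistent debug lines, sends OnBulletHitMessage to the hit actor, so hit notification is independent of the projectile.
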(event Custom|FireBullet
  (Utilities|FlowControl|Sequence
    (:then_0
      ;[0.5412 0.6136 1] Fire Bullet Event Call
      (bind _returnvalue (Game|SpawnActorfromClass "/Game/Blueprints/Bullet_Base.Bullet_Base_C" (Transformation|GetSocketTransform (Variables|Default|GetWeapon) "Muzzle" "RTS_World") "Undefined" 0 0))
      (Variables|Default|SetmyBullet _returnvalue)
      (bind _asthird_person_character (Utilities|Casting|CastToThirdPersonCharacter (Game|GetPlayerCharacter 0)))
      (Variables|/Script/Engine.MovementComponent|SetVelocity (Variables|/Game/Blueprints/Bullet_Base.Bullet_Base_C|GetProjectileMovement (Variables|Default|GetmyBullet)) (* (Math|Vector|GetForwardVector (Variables|/Game/ThirdPersonBP/Blueprints/ThirdPersonCharacter.ThirdPersonCharacter_C|GetFollowCamera _asthird_person_character)) (Variables|Default|GetBulletSpeed))))
    (:then_1
      ;[0.5412 0.6136 1] FireBullet LineTrace
      (bind _asthird_person_character_2 (Utilities|Casting|CastToThirdPersonCharacter (Game|GetPlayerCharacter 0)))
      (bind _outhit (Collision|LineTraceByChannel (Transformation|GetWorldLocation (Variables|/Game/ThirdPersonBP/Blueprints/ThirdPersonCharacter.ThirdPersonCharacter_C|GetFollowCamera _asthird_person_character_2)) (+ (Transformation|GetWorldLocation (Variables|/Game/ThirdPersonBP/Blueprints/ThirdPersonCharacter.ThirdPersonCharacter_C|GetFollowCamera _asthird_person_character_2)) (* (Math|Vector|GetForwardVector (Transformation|GetWorldRotation (Variables|/Game/ThirdPersonBP/Blueprints/ThirdPersonCharacter.ThirdPersonCharacter_C|GetFollowCamera _asthird_person_character_2))) (Variables|Default|GetLineTraceDistance))) "TraceTypeQuery1" false 0 "Persistent"))
      (Class|BulletHitIBP|OnBulletHit(Message) (.HitActor (Collision|BreakHitResult _outhit)) _outhit))))

(event EventBeginPlay)

(event Collision|EventActorBeginOverlap
  (params (OtherActor :type Actor%20Object%20Reference)))

(event EventTick
  (params (DeltaSeconds :type Float%20%28single-precision%29)))

(fn ConstructionScript)