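; Behavior tree task for zombie AI that copies the owning AI controller's target actor into a Blackboard object key.
; It casts the owner to AIController_Basic, falling back to AIController_Citizen, and calls Run on that controller before writing its TargetActor.
; Both branches then finish with success, while an owner of neither class leaves the task unfinished.
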(event EventReceiveExecute
  (params (OwnerActor :type Actor%20Object%20Reference))
  (bind _asaicontroller_basic (Utilities|Casting|CastToAIController_Basic OwnerActor)
    (:then
      (Default|Run _asaicontroller_basic)
      (Class|BTFunctionLibrary|SetBlackboardValueasObject (Variables|Default|GetTargetActorKey) (Variables|/Game/Blueprints/AI_Zombie/AIController_Basic.AIController_Basic_C|GetTargetActor _asaicontroller_basic)))
    (:CastFailed
      (bind _asaicontroller_citizen (Utilities|Casting|CastToAIController_Citizen OwnerActor))
      (Default|Run _asaicontroller_citizen)
      (Class|BTFunctionLibrary|SetBlackboardValueasObject (Variables|Default|GetTargetActorKey) (Variables|/Game/Blueprints/AI_Citizen/AIController_Citizen.AIController_Citizen_C|GetTargetActor _asaicontroller_citizen))))
  (AI|BehaviorTree|FinishExecute true))