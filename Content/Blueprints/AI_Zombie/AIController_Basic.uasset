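; Basic zombie AI controller that runs BT_Basic on a possessed SimpleAI pawn and forwards Walk, Run and Attack to it.
; Sight perception updates filter actors tagged "Human" through GetNearestTarget, whose distance check compares controller and pawn locations rather than the perceived actor's.
; The last result sets the CanSeePlayer blackboard key; when false, RecentlySeen is set and TargetActor's current location becomes the move-to location.
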(event OnPerceptionUpdated(AIPerception)
  (params (UpdatedActors :type Array%20of%20Actor%20Object%20References))
  ;[0.5412 0.6136 1] Check if AI can see player and Set BlackBoard value
  (for _array_element (Class|AIPerceptionComponent|GetPerceivedActors (Variables|Default|GetAIPerception) "/Script/AIModule.AISense_Sight")
    (bind _foundtarget (Utilities|GetNearestTarget _array_element)))
  (AI|Components|Blackboard|SetValueasBool (AI|GetBlackboard 0) (Variables|Default|GetCanSeePlayerKey) _foundtarget)
  (if (not _foundtarget)
    ;;[1 1 1] On Loose Sight
    (AI|Components|Blackboard|SetValueasBool (AI|GetBlackboard 0) (Variables|Default|GetRecentlySeenKey) true)
    (AI|Components|Blackboard|SetValueasVector (AI|GetBlackboard 0) (Variables|Default|GetMoveToLocationKey) (Transformation|GetActorLocation (Variables|Default|GetTargetActor)))))

(event Custom|Walk
  ;[0.5412 0.6136 1] Calling walk and run on SimpleAI
  (Default|Walk (Variables|Default|GetSimpleAI)))

(event Custom|Run
  ;[0.5412 0.6136 1] Calling walk and run on SimpleAI
  (Default|Run (Variables|Default|GetSimpleAI)))

(event Custom|Attack
  ;[0.5412 0.6136 1] Calling Attack on SimpleAI
  (Default|Attack (Variables|Default|GetSimpleAI)))

(event EventOnPossess
  (params (PossessedPawn :type Pawn%20Object%20Reference))
  ;[0.5412 0.6136 1] Run Behaviour Tree on AI
  (bind _assimple_ai (Utilities|Casting|CastToSimpleAI PossessedPawn))
  (Variables|Default|SetSimpleAI _assimple_ai)
  (AI|RunBehaviorTree "/Game/Blueprints/AI_Zombie/BT_Basic.BT_Basic"))

(fn ConstructionScript)