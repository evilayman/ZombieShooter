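; Zombie AI character that switches between walk and run speeds, melee-attacks and ragdolls when shot.
; Attack plays a montage-free animation and opens a brief timed damage window, during which socket-attached hand colliders send hit messages to overlapped actors.
; A bullet hit turns on blended full-body physics, applies an impulse at the struck bone, spawns an impact effect and unpossesses the controller.
; The old PawnSensing sight and hearing handlers are empty.
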(event OnSeePawn(PawnSensing)
  (params (Pawn :type Pawn%20Object%20Reference))
  ;[1 0.3737 0.3538] AI Vision Handling (OLD)
)

(event OnHearNoise(PawnSensing)
  (params (Instigator :type Pawn%20Object%20Reference) (Location :type Vector%20%28by%20ref%29 :default "0, 0, 0") (Volume :type Float%20%28single-precision%29))
  ;[1 0.3737 0.3538] AI Hearing Handling (OLD)
)

(event OnComponentBeginOverlap(Left)
  (params (OverlappedComponent :type Primitive%20Component%20Object%20Reference) (OtherActor :type Actor%20Object%20Reference) (OtherComp :type Primitive%20Component%20Object%20Reference) (OtherBodyIndex :type Integer) (bFromSweep :type Boolean) (SweepResult :type Hit%20Result%20Structure%20%28by%20ref%29))
  ;[0.5412 0.6136 1] Do Damage to Player from Hand Attacks
  (if (Variables|Default|GetIsAttacking)
    (Class|ZombieHitIBP|OnZombieHit(Message) OtherActor (Variables|Default|GetHandDamage))))

(event OnComponentBeginOverlap(Right)
  (params (OverlappedComponent :type Primitive%20Component%20Object%20Reference) (OtherActor :type Actor%20Object%20Reference) (OtherComp :type Primitive%20Component%20Object%20Reference) (OtherBodyIndex :type Integer) (bFromSweep :type Boolean) (SweepResult :type Hit%20Result%20Structure%20%28by%20ref%29))
  ;[0.5412 0.6136 1] Do Damage to Player from Hand Attacks
  (if (Variables|Default|GetIsAttacking)
    (Class|ZombieHitIBP|OnZombieHit(Message) OtherActor (Variables|Default|GetHandDamage))))

(event Custom|Walk
  ;[0.5412 0.6136 1] Movement Speed Setting
  (Variables|/Script/Engine.CharacterMovementComponent|SetMaxWalkSpeed (Variables|Character|GetCharacterMovement) (Variables|Default|GetWalkSpeed)))

(event Custom|Run
  ;[0.5412 0.6136 1] Movement Speed Setting
  (Variables|/Script/Engine.CharacterMovementComponent|SetMaxWalkSpeed (Variables|Character|GetCharacterMovement) (Variables|Default|GetRunSpeed)))

(event Custom|Attack
  ;[0.5412 0.6136 1] Play attack Animation
  (Components|Animation|PlayAnimation (Variables|Character|GetMesh) "/Game/Meshes/ZombieMaleMesh/Animations/Zombie_Attack.Zombie_Attack" false)
  (Components|Timeline|SetPlayRate (Variables|Character|GetMesh) 2.0)
  (Utilities|FlowControl|Delay 0.7)
  (Variables|Default|SetIsAttacking true)
  (Utilities|FlowControl|Delay 0.3)
  (Variables|Default|SetIsAttacking false)
  (Utilities|FlowControl|Delay 1.3)
  (Components|Animation|SetAnimationMode (Variables|Character|GetMesh) "AnimationBlueprint"))

(event EventOnBulletHit
  (params (Hit :type Hit%20Result%20Structure))
  (bind (_bblockinghit _binitialoverlap _time _distance _location _impactpoint _normal _impactnormal _physmat _hitactor _hitcomponent _hitbonename) (Collision|BreakHitResult Hit))
  ;[0.5412 0.6136 1] Bullet Hit Effect (Ragdoll)
  (Class|SkeletalMeshComponent|SetAllBodiesSimulatePhysics (Variables|Character|GetMesh) true)
  (Class|SkeletalMeshComponent|SetAllBodiesPhysicsBlendWeight (Variables|Character|GetMesh) 0.75 false)
  (Physics|AddImpulseatLocation (Variables|Character|GetMesh) (* (* _impactnormal -1.0) (Variables|Default|GetImpulseForce)) _impactpoint _hitbonename)
  (Effects|SpawnEmitteratLocation "/Game/InfinityBladeEffects/Effects/FX_Mobile/Impacts/P_Impact_Player_Fire_Weak.P_Impact_Player_Fire_Weak" _impactpoint)
  (Pawn|UnPossess (Pawn|GetController)))

(fn ConstructionScript
  (Transformation|AttachComponentToComponent (Variables|Default|GetLeft) (Variables|Character|GetMesh) "LeftHandSocket" "KeepRelative" "KeepRelative" "KeepRelative" true)
  (Transformation|AttachComponentToComponent (Variables|Default|GetRight) (Variables|Character|GetMesh) "RightHandSocket" "KeepRelative" "KeepRelative" "KeepRelative" true))