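; SimpleAI is a basic AI Blueprint that turns into a full-body ragdoll when a bullet hits it.
; OnBulletHit enables mesh collision and physics on all bodies, then applies an impulse at the impact point and bone, opposite the impact normal.
; Pawn sensing is stubbed: hearing noise prints a debug greeting and seeing a pawn does nothing.
; Disconnected nodes hold an unused chase-player move and a partial-body ragdoll variant.
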(event OnSeePawn(PawnSensing)
  (params (Pawn :type Pawn%20Object%20Reference)))

(event OnHearNoise(PawnSensing)
  (params (Instigator :type Pawn%20Object%20Reference) (Location :type Vector%20%28by%20ref%29 :default "0, 0, 0") (Volume :type Float%20%28single-precision%29))
  (Development|PrintString "Hello"))

(event EventOnBulletHit
  (params (Hit :type Hit%20Result%20Structure))
  (bind (_bblockinghit _binitialoverlap _time _distance _location _impactpoint _normal _impactnormal _physmat _hitactor _hitcomponent _hitbonename) (Collision|BreakHitResult Hit))
  (bind _mesh (Variables|Character|GetMesh))
  ;[0.5412 0.6136 1] Start Ragdoll on Hit
  (Collision|SetCollisionEnabled _mesh "QueryAndPhysics")
  (Class|SkeletalMeshComponent|SetAllBodiesSimulatePhysics _mesh true)
  (Class|SkeletalMeshComponent|SetAllBodiesPhysicsBlendWeight _mesh 1.0 false)
  (Physics|AddImpulseatLocation _mesh (* (* _impactnormal -1.0) (Variables|Default|GetImpulseForce)) _impactpoint _hitbonename))

(fn ConstructionScript)