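; AI controller for citizen NPCs that runs the Citizen_BT behavior tree on possession and forwards Walk and Run calls to the CitizenAI pawn.
; Each perception update scans sighted actors for the tagged player and the nearest tagged zombie, writing visibility flags to the Blackboard.
; When the player drops out of sight, it sets the recently-seen flag and stores the player's location as the move-to target.
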(event OnTargetPerceptionUpdated(AIPerception)
  (params (Actor :type Actor%20Object%20Reference) (Stimulus :type AI%20Stimulus%20Structure))
  ;[0.5412 0.6136 1] Check if AI can see player and Set BlackBoard value
  (Variables|Default|SetFoundPlayer false)
  (Variables|Default|SetFoundZombie false)
  (Variables|Default|SetTargetDistance 1e+05)
  (for _array_element (Class|AIPerceptionComponent|GetPerceivedActors (Variables|Default|GetAIPerception) "/Script/AIModule.AISense_Sight")
    (if (Actor|ActorHasTag _array_element "Player")
      (Variables|Default|SetFoundPlayer true)
      (Variables|Default|SetTargetActor _array_element)
      (else
        (Utilities|GetNearestZombie _array_element))))
  (AI|Components|Blackboard|SetValueasBool (AI|GetBlackboard 0) (Variables|Default|GetCanSeeZombieKey) (Variables|Default|GetFoundZombie))
  (AI|Components|Blackboard|SetValueasBool (AI|GetBlackboard 0) (Variables|Default|GetCanSeePlayerKey) (Variables|Default|GetFoundPlayer))
  (if (Variables|Default|GetFoundPlayer)
    ;;[1 1 1] On Loose Sight
    (if (not (Variables|Default|GetLastState))
      (Variables|Default|SetLastState true))
    (elif (Variables|Default|GetLastState)
      (Variables|Default|SetLastState false)
      (AI|Components|Blackboard|SetValueasBool (AI|GetBlackboard 0) (Variables|Default|GetRecentlySeenKey) true)
      (AI|Components|Blackboard|SetValueasVector (AI|GetBlackboard 0) (Variables|Default|GetMoveToLocationKey) (Transformation|GetActorLocation (Variables|Default|GetTargetActor))))))

(event Custom|Walk
  ;[0.5412 0.6136 1] Calling walk and run on SimpleAI
  (Default|Walk (Variables|Default|GetCitizenAI)))

(event Custom|Run
  ;[0.5412 0.6136 1] Calling walk and run on SimpleAI
  (Default|Run (Variables|Default|GetCitizenAI)))

(event EventOnPossess
  (params (PossessedPawn :type Pawn%20Object%20Reference))
  ;[0.5412 0.6136 1] Run Behaviour Tree on AI
  (bind _ascitizen_ai (Utilities|Casting|CastToCitizenAI PossessedPawn))
  (Variables|Default|SetCitizenAI _ascitizen_ai)
  (AI|RunBehaviorTree "/Game/Blueprints/AI_Citizen/Citizen_BT.Citizen_BT"))

(fn ConstructionScript)