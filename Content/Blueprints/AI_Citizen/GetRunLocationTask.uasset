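; Behavior tree task for citizen AI that picks a location to run to, away from the target zombie.
; It projects EscapeDistance from the owner along the direction away from the zombie, then finds a random reachable point within ReacheablePointRadius of that spot.
; The point is written to RandomLocationKey, and the task's success comes from the query's return value, which is evaluated again for that call.
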(event EventReceiveExecute
  (params (OwnerActor :type Actor%20Object%20Reference))
  (bind _returnvalue (Transformation|GetActorLocation OwnerActor))
  (bind _targetzombiekey (Variables|Default|GetTargetZombieKey))
  (bind _escapedistance (Variables|Default|GetEscapeDistance))
  (bind _reacheablepointradius (Variables|Default|GetReacheablePointRadius))
  (bind _returnvalue_2 (AI|BehaviorTree|GetBlackboardValueasActor _targetzombiekey))
  (bind _returnvalue_3 (Transformation|GetActorLocation _returnvalue_2))
  (bind _returnvalue_4 (Math|Vector|GetUnitDirection(Vector) _returnvalue_3 _returnvalue))
  (bind _returnvalue_5 (* _returnvalue_4 _escapedistance))
  (bind _returnvalue_6 (+ _returnvalue_5 _returnvalue))
  (bind (_randomlocation _returnvalue_7) (AI|Navigation|GetRandomReachablePointinRadius _returnvalue_6 _reacheablepointradius 0 0))
  (AI|BehaviorTree|SetBlackboardValueasVector (Variables|Default|GetRandomLocationKey) _randomlocation)
  (AI|BehaviorTree|FinishExecute _returnvalue_7))