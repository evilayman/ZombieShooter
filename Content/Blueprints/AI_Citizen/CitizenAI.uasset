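; CitizenAI is a citizen character Blueprint that can walk, run and be killed by zombies or bullets.
; Walk and Run events set the movement component's max speed.
; Both death events turn on ragdoll physics, unpossess the controller and replace the tags with Dead.
; Bullet hits also set a partial physics blend weight, push the struck bone opposite the impact normal and spawn an impact particle.
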(event Custom|Walk
  ;[0.5412 0.6136 1] Movement Speed Setting
  (Variables|/Script/Engine.CharacterMovementComponent|SetMaxWalkSpeed (Variables|Character|GetCharacterMovement) (Variables|Default|GetWalkSpeed)))

(event Custom|Run
  ;[0.5412 0.6136 1] Movement Speed Setting
  (Variables|/Script/Engine.CharacterMovementComponent|SetMaxWalkSpeed (Variables|Character|GetCharacterMovement) (Variables|Default|GetRunSpeed)))

(event EventOnZombieHit
  (params (damage :type Float%20%28single-precision%29))
  ;[0.5439 0.5266 1] On Zombie Hit
  (Class|SkeletalMeshComponent|SetAllBodiesSimulatePhysics (Variables|Character|GetMesh) true)
  (Pawn|UnPossess (Pawn|GetController))
  (Variables|Default|SetTags self (Utilities|Array|MakeArray "Dead")))

(event EventOnBulletHit
  (params (Hit :type Hit%20Result%20Structure))
  (bind (_bblockinghit _binitialoverlap _time _distance _location _impactpoint _normal _impactnormal _physmat _hitactor _hitcomponent _hitbonename) (Collision|BreakHitResult Hit))
  ;[0.5412 0.6136 1] Bullet Hit Effect (Ragdoll)
  (Class|SkeletalMeshComponent|SetAllBodiesSimulatePhysics (Variables|Character|GetMesh) true)
  (Class|SkeletalMeshComponent|SetAllBodiesPhysicsBlendWeight (Variables|Character|GetMesh) 0.75 false)
  (Physics|AddImpulseatLocation (Variables|Character|GetMesh) (* (* _impactnormal -1.0) (Variables|Default|GetImpulseForce)) _impactpoint _hitbonename)
  (Effects|SpawnEmitteratLocation "/Game/InfinityBladeEffects/Effects/FX_Mobile/Impacts/P_Impact_Player_Fire_Weak.P_Impact_Player_Fire_Weak" _impactpoint)
  (Pawn|UnPossess (Pawn|GetController))
  (Variables|Default|SetTags self (Utilities|Array|MakeArray "Dead")))

(fn ConstructionScript)