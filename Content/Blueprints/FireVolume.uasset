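; FireVolume is an actor that repeatedly damages the ThirdPersonCharacter while it stands inside.
; Begin and end overlap events cast to that character and toggle an InFire flag, with begin overlap supplying the damage target.
; Tick runs through a Delay of TimeForDamage as a repeating timer, then calls the character's TakeDamage with DamagePercent converted to a fraction if InFire is set.
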(event EventBeginPlay)

(event Collision|EventActorBeginOverlap
  (params (OtherActor :type Actor%20Object%20Reference))
  (bind _asthird_person_character (Utilities|Casting|CastToThirdPersonCharacter OtherActor))
  (Variables|Default|SetinFire true))

(event EventTick
  (params (DeltaSeconds :type Float%20%28single-precision%29))
  (Utilities|FlowControl|Delay (Variables|Default|GetTimeForDamage))
  (if (Variables|Default|GetinFire)
    (Default|TakeDamage (stale Collision|EventActorBeginOverlap _asthird_person_character) (/ (Variables|Default|GetDamagePercent) 1e+02))))

(event Collision|EventActorEndOverlap
  (params (OtherActor :type Actor%20Object%20Reference))
  (Utilities|Casting|CastToThirdPersonCharacter OtherActor)
  (Variables|Default|SetinFire false))

(fn ConstructionScript)